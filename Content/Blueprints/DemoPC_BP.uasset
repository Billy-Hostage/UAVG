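; Demo player controller that hosts a UAVG dialogue session through an on-screen UI.
; On BeginPlay it creates the DemoUI_BP widget, adds it to the viewport and initializes the UAVG component with it, starting the first line immediately.
; Pressing P sends a SimpleNextLine command to advance the component.
; The new-line and text-updated event handlers are empty.
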(event EventBeginPlay
  (bind _returnvalue (UserInterface|CreateWidget "/Game/Blueprints/DemoUI_BP.DemoUI_BP_C" self))
  (bind _output_get (Variables|Default|SetDemoUI _returnvalue))
  (UserInterface|Viewport|AddtoViewport _output_get 0)
  (Class|UAVGComponent|InitializeNew (Variables|Default|GetUAVG) _output_get self true))

(event EventOnNewLine
  (params (Info :type UAVG%20Actor%20Line%20Info%20Structure%20%28by%20ref%29)))

(event EventOnTextUpdated
  (params (Index :type Integer) (NewText :type Text%20%28by%20ref%29)))

(event Input|KeyboardEvents|P
  (params (Key :type Key%20Structure))
  (:Pressed
    (Class|UAVGComponent|Next (Variables|Default|GetUAVG) (Utilities|Struct|MakeUAVGComponentNextCommand "UNC_SimpleNextLine"))))

(fn ConstructionScript)